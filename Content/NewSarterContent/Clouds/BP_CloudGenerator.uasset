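; Cloud generator actor that fills a box-like region with drifting cloud meshes.
; The construction script uses a random stream to place randomly scaled, shadowless meshes from six variants under a CloudContainer rotated toward Endpoint.
; Tick moves each cloud along the container's local X at CloudSpeed.
; Clouds passing Endpoint.X recycle to the start with new random Y and Z offsets, creating a continuous flow.
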(event EventBeginPlay)

(event EventActorBeginOverlap
  (params (OtherActor :type Actor%20Object%20Reference)))

(event EventTick
  (params (DeltaSeconds :type Float%20%28single-precision%29))
  (bind _zrange (Variables|Default|GetZRange))
  (bind _yrange (Variables|Default|GetYRange))
  (bind _cloudspeed (Variables|Default|GetCloudSpeed))
  (bind _returnvalue (/ _yrange 2.0))
  (bind _returnvalue_2 (/ _zrange 2.0))
  (bind _returnvalue_3 (* DeltaSeconds _cloudspeed))
  (bind _returnvalue_4 (Math|Vector|MakeVector _returnvalue_3 0.0 0.0))
  (for _array_element (Variables|Default|GetClouds)
    (if (> (.X (Math|Vector|BreakVector (+ (Variables|/Script/Engine.SceneComponent|GetRelativeLocation _array_element) _returnvalue_4))) (.X (Math|Vector|BreakVector (Variables|Default|GetEndpoint))))
      (Transformation|SetRelativeLocation _array_element (Math|Vector|MakeVector 0.0 (Math|Random|RandomFloatinRangefromStream (- 0.0 _returnvalue) _returnvalue (Variables|Default|GetRandomStream)) (Math|Random|RandomFloatinRangefromStream (- 0.0 _returnvalue_2) _returnvalue_2 (Variables|Default|GetRandomStream))) false)
      (else
        (Transformation|AddRelativeLocation _array_element _returnvalue_4 false)))))

(fn ConstructionScript
  (bind _returnvalue (Transformation|GetActorLocation))
  (bind _randomstream (Variables|Default|GetRandomStream))
  (bind _zrange (Variables|Default|GetZRange))
  (bind _yrange (Variables|Default|GetYRange))
  (bind _scalerange (Variables|Default|GetScaleRange))
  (bind _returnvalue_2 (/ _yrange 2.0))
  (bind _returnvalue_3 (/ _zrange 2.0))
  (bind _returnvalue_4 (Math|Random|RandomFloatinRangefromStream 1.0 _scalerange _randomstream))
  (Utilities|FlowControl|Sequence
    (:then_0
      (for _index (range 1 (Variables|Default|GetCloudCount))
        (bind _returnvalue_5 (AddComponent|AddStaticMeshComponent true (Math|Transform|MakeTransform (Math|Vector|MakeVector (Math|Random|RandomFloatinRangefromStream 0.0 (Math|Vector|VectorLength (Variables|Default|GetEndpoint)) (Variables|Default|GetRandomStream)) (Math|Random|RandomFloatinRangefromStream (- 0.0 _returnvalue_2) _returnvalue_2 (Variables|Default|GetRandomStream)) (Math|Random|RandomFloatinRangefromStream (- 0.0 _returnvalue_3) _returnvalue_3 (Variables|Default|GetRandomStream))))))
        (Utilities|FlowControl|Sequence
          (:then_0
            (Utilities|Array|Add (Variables|Default|GetClouds) _returnvalue_5))
          (:then_1
            (Class|SceneComponent|Attachto _returnvalue_5 (Variables|Default|GetCloudContainer) "None" "KeepRelativeOffset" true))
          (:then_2
            (switch int (Math|Random|RandomIntegerinRangefromStream 0 5 (Variables|Default|GetRandomStream))
              (:Default
                (Components|StaticMesh|SetStaticMesh _returnvalue_5 "/Game/NewSarterContent/SM/Clouds/SM_CloudS_2.SM_CloudS_2"))
              (:0
                (Components|StaticMesh|SetStaticMesh _returnvalue_5 "/Game/NewSarterContent/SM/Clouds/SM_CloudL_1.SM_CloudL_1"))
              (:1
                (Components|StaticMesh|SetStaticMesh _returnvalue_5 "/Game/NewSarterContent/SM/Clouds/SM_CloudL_2.SM_CloudL_2"))
              (:2
                (Components|StaticMesh|SetStaticMesh _returnvalue_5 "/Game/NewSarterContent/SM/Clouds/SM_CloudM_1.SM_CloudM_1"))
              (:3
                (Components|StaticMesh|SetStaticMesh _returnvalue_5 "/Game/NewSarterContent/SM/Clouds/SM_CloudM_2.SM_CloudM_2"))
              (:4
                (Components|StaticMesh|SetStaticMesh _returnvalue_5 "/Game/NewSarterContent/SM/Clouds/SM_CloudS_1.SM_CloudS_1"))))
          (:then_3
            (Transformation|SetRelativeScale3D _returnvalue_5 (Math|Vector|MakeVector _returnvalue_4 _returnvalue_4 _returnvalue_4)))
          (:then_4
            (Transformation|SetRelativeRotation (Variables|Default|GetCloudContainer) (Math|Rotator|FindLookatRotation _returnvalue (+ _returnvalue (Variables|Default|GetEndpoint))) false))
          (:then_5
            (Rendering|SetCastShadow _returnvalue_5 false)))))))