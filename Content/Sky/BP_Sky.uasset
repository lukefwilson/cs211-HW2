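; BP_Sky is a sky actor whose colors and horizon falloff are configurable through its variables.
; Its construction script creates a dynamic instance of M_Sky on the Sky component and stores it as SkyMaterial.
; It then passes three color variables and the horizon falloff into that material's parameters, so the look is applied at construction.
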(fn ConstructionScript
  (Utilities|FlowControl|Sequence
    (:then_0
      (bind _returnvalue (Rendering|Material|CreateDynamicMaterialInstance (Variables|Default|GetSky) 0 "/Game/Materials/M_Sky.M_Sky" :!class /Script/Engine.PrimitiveComponent))
      (Variables|Default|SetSkyMaterial _returnvalue))
    (:then_1
      (Rendering|Material|SetVectorParameterValue (Variables|Default|GetSkyMaterial) "ColorA" (Variables|Default|GetColorA) :!class /Script/Engine.MaterialInstanceDynamic))
    (:then_2
      (Rendering|Material|SetVectorParameterValue (Variables|Default|GetSkyMaterial) "ColorB" (Variables|Default|GetColorB) :!class /Script/Engine.MaterialInstanceDynamic))
    (:then_3
      (Rendering|Material|SetVectorParameterValue (Variables|Default|GetSkyMaterial) "ColorPrincipal" (Variables|Default|GetColorPrincipal) :!class /Script/Engine.MaterialInstanceDynamic))
    (:then_4
      (Rendering|Material|SetScalarParameterValue (Variables|Default|GetSkyMaterial) "Horizon" (Variables|Default|GetHorizonFalloff) :!class /Script/Engine.MaterialInstanceDynamic))))