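; BP_ActorSpline is a spline-based placer that lines a path with GridCube child actors at a fixed spacing.
; The construction script steps along the spline by Space, adding a child actor component aligned to the spline's world location and rotation at each distance.
; Each cube gets a random mode, with the first forced to mode 3, plus a set rotation speed and zeroed sinusoidal movement speed.
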(event EventBeginPlay)

(event EventActorBeginOverlap
  (params (OtherActor :type Actor%20Object%20Reference)))

(event EventTick
  (params (DeltaSeconds :type Float%20%28single-precision%29)))

(fn ConstructionScript
  (bind _spline (Variables|Default|GetSpline))
  (for _index (range 0 (Math|Float|Floor (/ (Spline|GetSplineLength (Variables|Default|GetSpline)) (Variables|Default|GetSpace))))
    (bind _returnvalue (AddComponent|AddChildActorComponent false))
    (Transformation|SetWorldLocationAndRotation _returnvalue (Class|SplineComponent|GetWorldLocationatDistanceAlongSpline _spline (* _index (Variables|Default|GetSpace))) (Class|SplineComponent|GetWorldRotationatDistanceAlongSpline _spline (* _index (Variables|Default|GetSpace))) false)
    (bind _asgrid_cube (Utilities|Casting|CastToGridCube (Variables|/Script/Engine.ChildActorComponent|GetChildActor _returnvalue)))
    (Default|SetMode _asgrid_cube (Math|Random|RandomIntegerinRange 0 2))
    (Variables|/Game/Blueprints/BPC_Rotation.BPC_Rotation_C|SetSpeed (Variables|/Game/Blueprints/GridCube.GridCube_C|GetBPC_Rotation _asgrid_cube) 1.5)
    (Variables|/Game/Blueprints/BPC_SinasoidalMovement.BPC_SinasoidalMovement_C|SetSpeed (Variables|/Game/Blueprints/GridCube.GridCube_C|GetBPC_SinasoidalMovement _asgrid_cube) 0.0)
    (if (== _index 0)
      (Default|SetMode _asgrid_cube 3))))