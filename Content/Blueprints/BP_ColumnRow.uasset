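; BP_ColumnRow is a construction-script actor that builds a straight row of static mesh components from its origin toward an Endpoint offset.
; When Endpoint has a nonzero X, it attaches copies to Column at 60-unit intervals along local X, with the count derived from the vector's length.
; Column's relative rotation is set to look along Endpoint, swinging the whole row onto that direction.
; The event graph holds no runtime logic.
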(event EventBeginPlay)

(event EventActorBeginOverlap
  (params (OtherActor :type Actor%20Object%20Reference)))

(event EventTick
  (params (DeltaSeconds :type Float%20%28single-precision%29)))

(fn ConstructionScript
  (bind _returnvalue (Transformation|GetActorLocation))
  (bind _endpoint (Variables|Default|GetEndpoint))
  (if (Math|Vector|NotEqual(Vector) (* _endpoint "1.000000, 0, 0") "0.000000, 0, 0" 0.0)
    (for _index (range 1 (Math|Float|Floor (/ (Math|Vector|VectorLength _endpoint) 6e+01)))
      (bind _returnvalue_2 (AddComponent|AddStaticMeshComponent true))
      (Class|SceneComponent|Attachto _returnvalue_2 (Variables|Default|GetColumn) "None" "KeepRelativeOffset" true)
      (Transformation|SetRelativeLocation _returnvalue_2 (Math|Vector|MakeVector (* (Math|Conversions|ToFloat(Integer) _index) 6e+01) 0.0 0.0) false)
      (Transformation|SetRelativeRotation (Variables|Default|GetColumn) (Math|Rotator|FindLookatRotation _returnvalue (+ _returnvalue (Variables|Default|GetEndpoint))) false))))