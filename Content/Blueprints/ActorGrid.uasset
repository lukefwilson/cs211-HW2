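; Construction-script actor that fills a rectangular XY grid with child actors, expected to be GridCubes, sized by Endpoint and Spacing.
; Each child is attached to the root, placed by its grid index and given a uniform Scale.
; Cells get random height, rotation and GridCube mode, except the origin cube, which stays level and has its rotation frozen.
; Generation runs only when Endpoint is non-zero in X or Y; the event graph is empty.
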(event EventBeginPlay)

(event EventActorBeginOverlap
  (params (OtherActor :type Actor%20Object%20Reference)))

(event EventTick
  (params (DeltaSeconds :type Float%20%28single-precision%29)))

(fn ConstructionScript
  (bind _spacing (Variables|Default|GetSpacing))
  (bind _spacing_2 (Variables|Default|GetSpacing))
  (bind _rotationvariation (Variables|Default|GetRotationVariation))
  (bind _endpoint (Variables|Default|GetEndpoint))
  (bind (_x _y) (Math|Vector|BreakVector _endpoint))
  (if (Math|Vector|NotEqual(Vector) (* _endpoint "1.000000,1.000000, 0") "0.000000, 0, 0" 0.0)
    (for _index (range 0 (Math|Float|Floor (/ _x _spacing)))
      (for _index_2 (range 0 (Math|Float|Floor (/ _y _spacing)))
        (bind _returnvalue (AddComponent|AddChildActorComponent false))
        (if (or (!= _index 0) (!= _index_2 0))
          (Variables|Default|SetActorZ (Math|Random|RandomFloatinRange 0.0 (Variables|Default|GetHeightVariation)))
          (Variables|Default|SetActorRotation (Class|KismetMathLibrary|MakeRot (Math|Random|RandomFloatinRange 0.0 _rotationvariation) (Math|Random|RandomFloatinRange 0.0 _rotationvariation) (Math|Random|RandomFloatinRange 0.0 _rotationvariation)))
          (bind _asgrid_cube (Utilities|Casting|CastToGridCube (Variables|/Script/Engine.ChildActorComponent|GetChildActor _returnvalue))
            (:then
              (Default|SetMode _asgrid_cube (Math|Random|RandomIntegerinRange 0 2)))
            (:CastFailed
              _))
          (else
            (Variables|Default|SetActorZ 0.0)
            (Variables|Default|SetActorRotation "0, 0, 0")
            (bind _asgrid_cube_2 (Utilities|Casting|CastToGridCube (Variables|/Script/Engine.ChildActorComponent|GetChildActor _returnvalue))
              (:then
                (Default|FreezeRotation _asgrid_cube_2))
              (:CastFailed
                _))))
        (Class|SceneComponent|Attachto _returnvalue (Variables|Default|GetActorRoot) "None" "KeepRelativeOffset" true)
        (Transformation|SetRelativeLocation _returnvalue (Math|Vector|MakeVector (* _index _spacing_2) (* _index_2 _spacing_2) (Variables|Default|GetActorZ)) false)
        (Transformation|SetWorldScale3D _returnvalue (Math|Conversions|ToVector(Float) (Variables|Default|GetScale)))
        (Transformation|SetWorldRotation _returnvalue (Variables|Default|GetActorRotation) false)))))