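; BP_CelestialBody is an actor that orbits its Parent on one axis at a time, with a glow color showing the active axis.
; Tick rotates its offset from Parent by RotationMask times RotationSpeed, unscaled by delta time.
; SetMode picks the axis and color, flipping direction when that axis is already positive.
; Construction creates the dynamic glow material and requests a random mode; Target raises or lowers emissive strength.
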(event Custom|RotateZ
  (Rendering|Material|SetVectorParameterValue (Variables|Default|GetGlowMaterial) "Color" "(R=1.000000,G=0.029149,B=0.000000,A=1.000000)" :!class /Script/Engine.MaterialInstanceDynamic)
  (if (Math|Vector|Equal(Vector) (Variables|Default|GetRotationMask) "0.000000,0.000000,1.000000" 0.0001)
    (Variables|Default|SetRotationMask "0.000000, 0,-1.000000")
    (else
      (Variables|Default|SetRotationMask "0.000000,0.000000,1.000000"))))

(event Custom|RotateX
  (Rendering|Material|SetVectorParameterValue (Variables|Default|GetGlowMaterial) "Color" "(R=0.000000,G=0.625516,B=1.000000,A=1.000000)" :!class /Script/Engine.MaterialInstanceDynamic)
  (if (Math|Vector|Equal(Vector) (Variables|Default|GetRotationMask) "1.000000, 0, 0" 0.0001)
    (Variables|Default|SetRotationMask "-1.000000, 0, 0")
    (else
      (Variables|Default|SetRotationMask "1.000000, 0, 0"))))

(event Custom|RotateY
  (Rendering|Material|SetVectorParameterValue (Variables|Default|GetGlowMaterial) "Color" "(R=1.000000,G=0.672219,B=0.000000,A=1.000000)" :!class /Script/Engine.MaterialInstanceDynamic)
  (if (Math|Vector|Equal(Vector) (Variables|Default|GetRotationMask) "0.000000,1.000000, 0" 0.0001)
    (Variables|Default|SetRotationMask "0.000000,-1.000000, 0")
    (else
      (Variables|Default|SetRotationMask "0.000000,1.000000, 0"))))

(event EventTick
  (params (DeltaSeconds :type Float%20%28single-precision%29))
  (bind _rotationspeed (Variables|Default|GetRotationSpeed))
  (bind _rotationmask (Variables|Default|GetRotationMask))
  (bind _parent (Variables|Default|GetParent))
  (bind _returnvalue (* _rotationmask _rotationspeed))
  (Utilities|IsValid _parent
    (:Is%20Valid
      (Transformation|SetActorLocation (+ (Math|Vector|RotateVector (- (Transformation|GetActorLocation) (Transformation|GetActorLocation _parent)) (Math|Rotator|MakeRotator (.x _returnvalue) (.y _returnvalue) (.z _returnvalue))) (Transformation|GetActorLocation (Variables|Default|GetParent))) false))))

(event EventSetMode
  (params (Mode :type Integer))
  (Utilities|IsValid (Variables|Default|GetParent)
    (:Is%20Valid
      (switch int Mode
        (:0
          (CallFunction|RotateX))
        (:1
          (CallFunction|RotateY))
        (:2
          (CallFunction|RotateZ))))))

(event EventTarget
  (params (targeted :type Boolean))
  (bind _glowmaterial (Variables|Default|GetGlowMaterial))
  (bind _output_get (Variables|Default|SetTargeted targeted))
  (if _output_get
    (Rendering|Material|SetScalarParameterValue _glowmaterial "EmisiveStrength" 6.0 :!class /Script/Engine.MaterialInstanceDynamic)
    (else
      (Rendering|Material|SetScalarParameterValue _glowmaterial "EmisiveStrength" 2.0 :!class /Script/Engine.MaterialInstanceDynamic))))

(fn ConstructionScript
  (Components|StaticMesh|SetStaticMesh (Variables|Default|GetMesh))
  (bind _returnvalue (Rendering|Material|CreateDynamicMaterialInstance (Variables|Default|GetMaterial) :!class /Script/Engine.KismetMaterialLibrary))
  (bind _output_get (Variables|Default|SetGlowMaterial _returnvalue))
  (Rendering|Material|SetMaterial 0 _output_get)
  (CallFunction|SetMode (Math|Random|RandomIntegerinRange 0 2)))