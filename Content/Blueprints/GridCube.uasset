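; GridCube is a glowing cube that changes spin axis and color on command and brightens while targeted.
; The construction script creates a dynamic emissive material, whose strength Target adjusts.
; SetMode routes to X, Y, Z or freeze events, each setting a color and the rotation component's RotationMask.
; Selecting an axis already spinning in the positive direction reverses it, while freeze zeroes the mask and turns the glow white.
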(event Custom|RotateZ
  (bind _bpc_rotation (Variables|Default|GetBPC_Rotation))
  (Rendering|Material|SetVectorParameterValue (Variables|Default|GetGlowMaterial) "Color" "(R=1.000000,G=0.029149,B=0.000000,A=1.000000)" :!class /Script/Engine.MaterialInstanceDynamic)
  (if (Math|Vector|Equal(Vector) (Variables|/Game/Blueprints/BPC_Rotation.BPC_Rotation_C|GetRotationMask _bpc_rotation) "0.000000,0.000000,1.000000" 0.0001)
    (Variables|/Game/Blueprints/BPC_Rotation.BPC_Rotation_C|SetRotationMask _bpc_rotation "0.000000,0.000000,-1.000000")
    (else
      (Variables|/Game/Blueprints/BPC_Rotation.BPC_Rotation_C|SetRotationMask _bpc_rotation "0.000000,0.000000,1.000000"))))

(event Custom|RotateX
  (bind _bpc_rotation (Variables|Default|GetBPC_Rotation))
  (Rendering|Material|SetVectorParameterValue (Variables|Default|GetGlowMaterial) "Color" "(R=0.000000,G=0.625516,B=1.000000,A=1.000000)" :!class /Script/Engine.MaterialInstanceDynamic)
  (if (Math|Vector|Equal(Vector) (Variables|/Game/Blueprints/BPC_Rotation.BPC_Rotation_C|GetRotationMask _bpc_rotation) "1.000000, 0, 0" 0.0001)
    (Variables|/Game/Blueprints/BPC_Rotation.BPC_Rotation_C|SetRotationMask _bpc_rotation "-1.000000,0.000000, 0")
    (else
      (Variables|/Game/Blueprints/BPC_Rotation.BPC_Rotation_C|SetRotationMask _bpc_rotation "1.000000,0.000000, 0"))))

(event Custom|RotateY
  (bind _bpc_rotation (Variables|Default|GetBPC_Rotation))
  (Rendering|Material|SetVectorParameterValue (Variables|Default|GetGlowMaterial) "Color" "(R=1.000000,G=0.672219,B=0.000000,A=1.000000)" :!class /Script/Engine.MaterialInstanceDynamic)
  (if (Math|Vector|Equal(Vector) (Variables|/Game/Blueprints/BPC_Rotation.BPC_Rotation_C|GetRotationMask _bpc_rotation) "0.000000,1.000000, 0" 0.0001)
    (Variables|/Game/Blueprints/BPC_Rotation.BPC_Rotation_C|SetRotationMask _bpc_rotation "0.000000,-1.000000, 0")
    (else
      (Variables|/Game/Blueprints/BPC_Rotation.BPC_Rotation_C|SetRotationMask _bpc_rotation "0.000000,1.000000, 0"))))

(event Custom|FreezeRotation
  (Rendering|Material|SetVectorParameterValue (Variables|Default|GetGlowMaterial) "Color" "(R=1.000000,G=1.000000,B=1.000000,A=1.000000)" :!class /Script/Engine.MaterialInstanceDynamic)
  (Variables|/Game/Blueprints/BPC_Rotation.BPC_Rotation_C|SetRotationMask (Variables|Default|GetBPC_Rotation) "0.000000,0.000000, 0"))

(event EventTarget
  (params (targeted :type Boolean))
  (bind _glowmaterial (Variables|Default|GetGlowMaterial))
  (bind _output_get (Variables|Default|SetTargeted targeted))
  (if _output_get
    (Rendering|Material|SetScalarParameterValue _glowmaterial "EmisiveStrength" 6.0 :!class /Script/Engine.MaterialInstanceDynamic)
    (else
      (Rendering|Material|SetScalarParameterValue _glowmaterial "EmisiveStrength" 2.0 :!class /Script/Engine.MaterialInstanceDynamic))))

(event EventSetMode
  (params (Mode :type Integer))
  (switch int Mode
    (:0
      (CallFunction|RotateX))
    (:1
      (CallFunction|RotateY))
    (:2
      (CallFunction|RotateZ))
    (:3
      (CallFunction|FreezeRotation))))

(fn ConstructionScript
  (bind _returnvalue (Rendering|Material|CreateDynamicMaterialInstance "/Game/Materials/New/M_Emisive.M_Emisive" :!class /Script/Engine.KismetMaterialLibrary))
  (bind _output_get (Variables|Default|SetGlowMaterial _returnvalue))
  (Rendering|Material|SetMaterial 0 _output_get))